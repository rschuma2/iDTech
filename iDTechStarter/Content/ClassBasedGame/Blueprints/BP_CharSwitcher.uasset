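; BP_CharSwitcher is a trigger that swaps the player's character class in a class-based game.
; When a ClassBasedCharacter overlaps its Box, it spawns the Blue, Red or Green character chosen by SelectedCharacter at the Arrow's transform.
; Player controller 0 possesses the new character and the overlapping one is destroyed.
; A CanSwitch flag blocks repeat switches until a short delay after an overlap ends.
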(event OnComponentBeginOverlap(Box)
  (params (OverlappedComponent :type Primitive%20Component%20Object%20Reference) (OtherActor :type Actor%20Object%20Reference) (OtherComp :type Primitive%20Component%20Object%20Reference) (OtherBodyIndex :type Integer) (bFromSweep :type Boolean) (SweepResult :type Hit%20Result%20Structure%20%28by%20ref%29))
  (bind _arrow (Variables|Default|GetArrow))
  (bind _returnvalue (Transformation|GetWorldTransform _arrow))
  (if (and (Utilities|ClassIsChildOf (Utilities|GetClass OtherActor) "/Game/ClassBasedGame/Blueprints/Characters/ClassBasedCharacter.ClassBasedCharacter_C") (Variables|Default|GetbCanSwitch))
    (Variables|Default|SetbCanSwitch false)
    (switch name (Variables|Default|GetSelectedCharacter)
      (:Blue
        (bind _returnvalue_2 (Game|SpawnActorfromClass "/Game/ClassBasedGame/Blueprints/Characters/BlueCharacter.BlueCharacter_C" _returnvalue "Undefined" 0 0))
        (Pawn|Possess (Game|GetPlayerController 0) _returnvalue_2)
        (Actor|DestroyActor OtherActor))
      (:Red
        (bind _returnvalue_3 (Game|SpawnActorfromClass "/Game/ClassBasedGame/Blueprints/Characters/RedCharacter.RedCharacter_C" _returnvalue "Undefined" 0 0))
        (Pawn|Possess (Game|GetPlayerController 0) _returnvalue_3)
        (Actor|DestroyActor OtherActor))
      (:Green
        (bind _returnvalue_4 (Game|SpawnActorfromClass "/Game/ClassBasedGame/Blueprints/Characters/GreenCharacter.GreenCharacter_C" _returnvalue "Undefined" 0 0))
        (Pawn|Possess (Game|GetPlayerController 0) _returnvalue_4)
        (Actor|DestroyActor OtherActor)))))

(event OnComponentEndOverlap(Box)
  (params (OverlappedComponent :type Primitive%20Component%20Object%20Reference) (OtherActor :type Actor%20Object%20Reference) (OtherComp :type Primitive%20Component%20Object%20Reference) (OtherBodyIndex :type Integer))
  (Utilities|FlowControl|Delay 2.0)
  (Variables|Default|SetbCanSwitch true))

(fn ConstructionScript)