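; BP_PickupBase is a health pickup for the class-based game, apparently meant as a base pickup.
; When a ClassBasedCharacter overlaps its sphere, it calls ChangeHealth with HealAmount and destroys itself.
; The heal targets player character 0 rather than the overlapping actor, so any character of that class triggers healing for that player.
; An older direct Health addition with a debug print remains disconnected.
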(event OnComponentBeginOverlap(Sphere1)
  (params (OverlappedComponent :type Primitive%20Component%20Object%20Reference) (OtherActor :type Actor%20Object%20Reference) (OtherComp :type Primitive%20Component%20Object%20Reference) (OtherBodyIndex :type Integer) (bFromSweep :type Boolean) (SweepResult :type Hit%20Result%20Structure%20%28by%20ref%29))
  (if (Utilities|ClassIsChildOf (Utilities|GetClass OtherActor) "/Game/ClassBasedGame/Blueprints/Characters/ClassBasedCharacter.ClassBasedCharacter_C")
    (bind _asclass_based_character (Utilities|Casting|CastToClassBasedCharacter (Game|GetPlayerCharacter 0)))
    (Default|ChangeHealth _asclass_based_character (Variables|Default|GetHealAmount))
    (Actor|DestroyActor)))

(event EventBeginPlay)

(event Collision|EventActorBeginOverlap
  (params (OtherActor :type Actor%20Object%20Reference)))

(event EventTick
  (params (DeltaSeconds :type Float%20%28single-precision%29)))

(fn ConstructionScript)