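; Base enemy for the class-based game: a suicide bomber that chases the player and explodes on reaching them.
; Pawn sensing triggers an AI MoveTo toward the seen class-based character; on arrival it deals radial damage and destroys itself.
; Incoming damage lowers health and can destroy it with explosion effects.
; When the last enemy is destroyed, it increments the game instance's level index and opens that level.
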(event Custom|OnSeePawn
  (params (Pawn :type Pawn%20Object%20Reference))
  (Variables|Default|SetSeenPawn Pawn)
  (CallFunction|HuntPlayer))

(event Custom|HuntPlayer
  (bind _returnvalue (Transformation|GetActorLocation))
  (bind _asclass_based_character (Utilities|Casting|CastToClassBasedCharacter (Variables|Default|GetSeenPawn)))
  (AI|AIMoveTo self "0, 0, 0" _asclass_based_character 1e+02 false
    (:OnSuccess
      (Effects|SpawnEmitteratLocation "/Game/StarterContent/Particles/P_Explosion.P_Explosion" _returnvalue)
      (Audio|PlaySound2D "/Game/StarterContent/Audio/Explosion01.Explosion01" 1.0 1.0 0.0 0 0)
      (Game|Damage|ApplyRadialDamage (Variables|Default|GetDamage) _returnvalue (Variables|Default|GetDamageRadius) 0 0 0 0 false "ECC_Visibility")
      (Actor|DestroyActor))))

(event EventBeginPlay
  (EventDispatchers|BindEventtoOnSeePawn (Variables|Default|GetPawnSensing) (delegate Custom|OnSeePawn)))

(event Game|Damage|EventAnyDamage
  (params (Damage :type Float%20%28single-precision%29) (DamageType :type Damage%20Type%20Object%20Reference) (InstigatedBy :type Controller%20Object%20Reference) (DamageCauser :type Actor%20Object%20Reference))
  (bind _returnvalue (Transformation|GetActorLocation))
  (Variables|Default|SetHealth (- (Variables|Default|GetHealth) (Math|Float|Truncate Damage)))
  (if (<= (- (Variables|Default|GetHealth) (Math|Float|Truncate Damage)) 0)
    (Effects|SpawnEmitteratLocation "/Game/StarterContent/Particles/P_Explosion.P_Explosion" _returnvalue)
    (Audio|PlaySoundatLocation "/Game/StarterContent/Audio/Explosion01.Explosion01" _returnvalue "0, 0, 0" 1.0 1.0 0.0 0 0 0)
    (Actor|DestroyActor)))

(event EventDestroyed
  (bind _outactors (Actor|GetAllActorsOfClass "BP_EnemyBase_C"))
  (if (<= (Utilities|Array|Length _outactors) 1)
    (bind _asgi_class_based (Utilities|Casting|CastToGI_ClassBased (Game|GetGameInstance)))
    (Variables|/Game/ClassBasedGame/Blueprints/GI_ClassBased.GI_ClassBased_C|SetCurrentLevel _asgi_class_based (+ (Variables|/Game/ClassBasedGame/Blueprints/GI_ClassBased.GI_ClassBased_C|GetCurrentLevel _asgi_class_based) 1))
    (Game|OpenLevel(byName) (Utilities|Array|Get(acopy) (Variables|/Game/ClassBasedGame/Blueprints/GI_ClassBased.GI_ClassBased_C|GetLevels _asgi_class_based) (Variables|/Game/ClassBasedGame/Blueprints/GI_ClassBased.GI_ClassBased_C|GetCurrentLevel _asgi_class_based)))))

(fn ConstructionScript)