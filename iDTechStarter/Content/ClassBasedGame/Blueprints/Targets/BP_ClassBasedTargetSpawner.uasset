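; BP_ClassBasedTargetSpawner is a destructible actor that keeps producing BP_ClassBasedTarget actors for the class-based game.
; A looping timer from BeginPlay spawns a target slightly above the spawner every second, and clears itself once GM_ClassBased reports game over.
; AnyDamage lowers Health and destroys the spawner, re-subtracting the damage in its zero-or-below check.
; MoveTarget is an inactive stub with a zero offset and an unconnected timer.
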(event Custom|HandleTargetSpawning
  (bind _self self)
  (bind _returnvalue (Transformation|GetActorTransform _self))
  ;[1 1 1] Handle Target Spawning
  (bind _asgm_class_based (Utilities|Casting|CastToGM_ClassBased (Game|GetGameMode)))
  (if (Variables|/Game/ClassBasedGame/Blueprints/GM_ClassBased.GM_ClassBased_C|GetbIsGameOver _asgm_class_based)
    (Utilities|Time|ClearandInvalidateTimerbyHandle (Variables|Default|GetSpawnerHandle))
    (else
      (Game|SpawnActorfromClass "/Game/ClassBasedGame/Blueprints/Targets/BP_ClassBasedTarget.BP_ClassBasedTarget_C" (Math|Transform|MakeTransform (Math|Vector|MakeVector (.x (.location _returnvalue)) (.y (.location _returnvalue)) (+ (.z (.location _returnvalue)) 5e+01)) (.rotation _returnvalue) (.scale _returnvalue)) "Undefined" 0 0))))

(event Custom|MoveTarget
  (Transformation|AddActorWorldOffset "0, 0, 0"))

(event EventBeginPlay
  (bind _returnvalue (Utilities|Time|SetTimerbyEvent (delegate Custom|HandleTargetSpawning) 1.0 true))
  (Variables|Default|SetSpawnerHandle _returnvalue))

(event Game|Damage|EventAnyDamage
  (params (Damage :type Float%20%28single-precision%29) (DamageType :type Damage%20Type%20Object%20Reference) (InstigatedBy :type Controller%20Object%20Reference) (DamageCauser :type Actor%20Object%20Reference))
  (Variables|Default|SetHealth (- (Variables|Default|GetHealth) (Math|Float|Truncate Damage)))
  (if (<= (- (Variables|Default|GetHealth) (Math|Float|Truncate Damage)) 0)
    (Actor|DestroyActor)))

(fn ConstructionScript)