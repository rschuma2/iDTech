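; GM_ClassBased is the game mode for the class-based game, running a timed round that ends in a game-over screen.
; On BeginPlay it sets game-only input, shows the W_CBHUD widget and starts a looping one-second timer that counts RoundTime down.
; When time runs out, it shows W_CBGameOver with UI-only input and a mouse cursor, sets IsGameOver and clears the timer.
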(event Custom|CountTimerDown
  (bind _returnvalue (Game|GetPlayerController 0))
  (bind _result (Math|Integer|DecrementInt (Variables|Default|GetRoundTime))
    (:%20%20
      (if (<= _result 0)
        (bind _returnvalue_2 (UserInterface|CreateWidget "/Game/ClassBasedGame/Widgets/W_CBGameOver.W_CBGameOver_C" _returnvalue))
        (UserInterface|Viewport|AddtoViewport _returnvalue_2 0)
        (Input|SetInputModeUIOnly _returnvalue _returnvalue_2 "DoNotLock")
        (Variables|/Script/Engine.PlayerController|SetbShowMouseCursor _returnvalue true)
        (Variables|Default|SetbIsGameOver true)
        (Utilities|Time|ClearandInvalidateTimerbyHandle (Variables|Default|GetCountTimerDownHandle))))))

(event Custom|HandleCountdownTimer
  (CallFunction|CountTimerDown))

(event EventBeginPlay
  (Utilities|FlowControl|Sequence
    (:then_0
      (Input|SetInputModeGameOnly (Game|GetPlayerController 0))
      (bind _returnvalue (UserInterface|CreateWidget "/Game/ClassBasedGame/Widgets/W_CBHUD.W_CBHUD_C" (Game|GetPlayerController 0)))
      (UserInterface|Viewport|AddtoViewport _returnvalue 0)
      (bind _returnvalue_2 (Utilities|Time|SetTimerbyEvent (delegate Custom|HandleCountdownTimer) 1.0 true))
      (Variables|Default|SetCountTimerDownHandle _returnvalue_2))))

(fn ConstructionScript)