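; BP_AIHide is an AI pawn that reports what it perceives to its AIC_Hide controller.
; Perception updates store the sensed actor and set the controller's target and line-of-sight keys.
; Losing sight clears line of sight immediately but starts an AttentionSpan timer that forgets the target on expiry unless something is sensed again first.
; Both perception events also print a debug "Hello".
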(event OnPerceptionUpdated(AIPerception)
  (params (UpdatedActors :type Array%20of%20Actor%20Object%20References))
  (Development|PrintString "Hello"))

(event OnTargetPerceptionUpdated(AIPerception)
  (params (Actor :type Actor%20Object%20Reference) (Stimulus :type AI%20Stimulus%20Structure))
  (bind _returnvalue (Pawn|GetController))
  (bind _asaic_hide (Utilities|Casting|CastToAIC_Hide _returnvalue))
  (Development|PrintString "Hello")
  (Variables|Default|SetPerceivedActor Actor)
  (if (.bsuccessfullysensed Stimulus)
    ;[1 1 1] Sees player successfully
    (Utilities|Time|ClearandInvalidateTimerbyHandle (Variables|Default|GetTargetLostHandle))
    (Default|UpdateTargetActorKey _asaic_hide (Variables|Default|GetPerceivedActor))
    (Default|UpdateHasLineOfSightKey _asaic_hide true)
    (else
      ;[1 1 1] Loses sight of player
      (bind _returnvalue_2 (Utilities|Time|SetTimerbyEvent (delegate Custom|TargetLost) (Variables|Default|GetAttentionSpan)))
      (Variables|Default|SetTargetLostHandle _returnvalue_2)
      (Default|UpdateHasLineOfSightKey (.AsAIC%20Hide (Utilities|Casting|CastToAIC_Hide (Pawn|GetController))) false))))

(event Custom|TargetLost
  ;[1 1 1] Loses sight of player
  (Variables|Default|SetPerceivedActor 0)
  (Default|UpdateTargetActorKey (.AsAIC%20Hide (Utilities|Casting|CastToAIC_Hide (Pawn|GetController)))))

(fn ConstructionScript)