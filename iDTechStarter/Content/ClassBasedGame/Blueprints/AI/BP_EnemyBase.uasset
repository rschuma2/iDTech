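; BP_EnemyBase is a suicide-bomber enemy that hunts the player and explodes on reaching them.
; Pawn sensing stores any seen pawn, and if it casts to ClassBasedCharacter the enemy uses AI MoveTo to chase it.
; When the move succeeds, it spawns an explosion effect and sound, applies radial damage around itself, and destroys itself.
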(event Custom|OnSeePawn
  (params (Pawn :type Pawn%20Object%20Reference))
  (Variables|Default|SetSeenPawn Pawn)
  (CallFunction|HuntPlayer))

(event Custom|HuntPlayer
  (bind _returnvalue (Transformation|GetActorLocation))
  (bind _asclass_based_character (Utilities|Casting|CastToClassBasedCharacter (Variables|Default|GetSeenPawn)))
  (AI|AIMoveTo self "0, 0, 0" _asclass_based_character 1e+02 false
    (:OnSuccess
      (Effects|SpawnEmitteratLocation "/Game/StarterContent/Particles/P_Explosion.P_Explosion" _returnvalue)
      (Audio|PlaySound2D "/Game/StarterContent/Audio/Explosion01.Explosion01" 1.0 1.0 0.0 0 0)
      (Game|Damage|ApplyRadialDamage 5e+01 _returnvalue 2.5e+02 0 0 0 0 false "ECC_Visibility")
      (Actor|DestroyActor))))

(event EventBeginPlay
  (EventDispatchers|BindEventtoOnSeePawn (Variables|Default|GetPawnSensing) (delegate Custom|OnSeePawn)))

(fn ConstructionScript)