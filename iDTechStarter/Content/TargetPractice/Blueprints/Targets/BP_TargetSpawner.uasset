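; BP_TargetSpawner spawns BP_Target actors at its location for the target practice mode.
; A looping one-second timer, started on BeginPlay, spawns each target slightly above the spawner with the same rotation and scale.
; Each tick of that timer checks IsGameOver on GM_TargetPractice and clears the timer once the game ends.
; A MoveTarget event exists with a zero offset, but its timer is never connected.
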(event Custom|HandleTargetSpawning
  (bind _self self)
  (bind _returnvalue (Transformation|GetActorTransform _self))
  ;[1 1 1] Handle Target Spawning
  (bind _asgm_target_practice (Utilities|Casting|CastToGM_TargetPractice (Game|GetGameMode)))
  (if (Variables|/Game/TargetPractice/Blueprints/GM_TargetPractice.GM_TargetPractice_C|GetbIsGameOver _asgm_target_practice)
    (Utilities|Time|ClearandInvalidateTimerbyHandle (Variables|Default|GetSpawnerHandle))
    (else
      (Game|SpawnActorfromClass "/Game/TargetPractice/Blueprints/Targets/BP_Target.BP_Target_C" (Math|Transform|MakeTransform (Math|Vector|MakeVector (.x (.location _returnvalue)) (.y (.location _returnvalue)) (+ (.z (.location _returnvalue)) 5e+01)) (.rotation _returnvalue) (.scale _returnvalue)) "Undefined" 0 0))))

(event Custom|MoveTarget
  (Transformation|AddActorWorldOffset "0, 0, 0"))

(event EventBeginPlay
  (bind _returnvalue (Utilities|Time|SetTimerbyEvent (delegate Custom|HandleTargetSpawning) 1.0 true))
  (Variables|Default|SetSpawnerHandle _returnvalue))

(fn ConstructionScript)