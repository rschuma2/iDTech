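; BP_Target is a short-lived shooting target that launches upward with random sideways impulse and removes itself on a timer.
; Construction randomizes sphere scale and, in a separate roll, a Modifier that divides the base Score at BeginPlay.
; Projectile hits play explosion effects, award Score to the player character, and increment GM_ClassBased kills, printing whether the kill limit is reached.
; Hits leave the target alive until the timer expires.
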(event OnComponentHit(Sphere)
  (params (HitComponent :type Primitive%20Component%20Object%20Reference) (OtherActor :type Actor%20Object%20Reference) (OtherComp :type Primitive%20Component%20Object%20Reference) (NormalImpulse :type Vector :default "0, 0, 0") (Hit :type Hit%20Result%20Structure%20%28by%20ref%29))
  (Utilities|Casting|CastToTargetPracticeProjectile OtherActor)
  (Effects|SpawnEmitteratLocation "/Game/StarterContent/Particles/P_Explosion.P_Explosion" (Transformation|GetWorldLocation (Variables|Default|GetSphere)))
  (Audio|PlaySound2D "/Game/StarterContent/Audio/Explosion01.Explosion01" 1.0 1.0 0.0 0 0)
  (bind _astarget_practice_character (Utilities|Casting|CastToTargetPracticeCharacter (Game|GetPlayerCharacter 0)))
  (Default|IncreaseScore _astarget_practice_character (Variables|Default|GetScore))
  (bind _asgm_class_based (Utilities|Casting|CastToGM_ClassBased (Game|GetGameMode)))
  (bind _result (Math|Integer|IncrementInt (Variables|/Game/ClassBasedGame/Blueprints/GM_ClassBased.GM_ClassBased_C|GetKills _asgm_class_based))
    (:%20%20
      (if (>= _result (Variables|/Game/ClassBasedGame/Blueprints/GM_ClassBased.GM_ClassBased_C|GetKillLimit _asgm_class_based))
        (Development|PrintString "Victory")
        (else
          (Development|PrintString "Not yet"))))))

(event Custom|DeleteTarget
  (Actor|DestroyActor))

(event EventBeginPlay
  (Physics|AddImpulse (Variables|Default|GetSphere) (Math|Vector|MakeVector (Math|Random|RandomFloatinRange -1.6e+04 1.6e+04) (Math|Random|RandomFloatinRange -1.6e+04 1.6e+04) 1e+05) "None" false)
  (Variables|Default|SetScore (Math|Float|Floor (/ (Math|Conversions|ToFloat(Integer) (Variables|Default|GetScore)) (Variables|Default|GetModifier))))
  (Utilities|Time|SetTimerbyEvent (delegate Custom|DeleteTarget) 2.0))

(fn ConstructionScript
  (bind _returnvalue (Math|Random|RandomFloatinRange 0.5 1.2))
  (bind _sphere (Variables|Default|GetSphere))
  (Variables|Default|SetModifier _returnvalue)
  (Transformation|SetWorldScale3D _sphere (* (Transformation|GetWorldScale _sphere) _returnvalue)))