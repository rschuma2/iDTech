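; BP_Car is a moving car hazard in Target Practice that launches and damages the player on contact.
; On BeginPlay it picks a random speed, scales its damage by it, and starts a fast looping timer that offsets it along Direction without sweeping.
; Box overlap with a TargetPracticeCharacter launches them along the root-to-arrow direction with an upward boost, then subtracts the damage from their health.
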(event OnComponentBeginOverlap(Box)
  (params (OverlappedComponent :type Primitive%20Component%20Object%20Reference) (OtherActor :type Actor%20Object%20Reference) (OtherComp :type Primitive%20Component%20Object%20Reference) (OtherBodyIndex :type Integer) (bFromSweep :type Boolean) (SweepResult :type Hit%20Result%20Structure%20%28by%20ref%29))
  (bind _arrow (Variables|Default|GetArrow))
  (bind _defaultsceneroot (Variables|Default|GetDefaultSceneRoot))
  (bind _returnvalue (Transformation|GetWorldLocation _defaultsceneroot))
  (bind _returnvalue_2 (Transformation|GetWorldLocation _arrow))
  (bind _returnvalue_3 (Math|Vector|GetUnitDirection(Vector) _returnvalue _returnvalue_2))
  (bind _returnvalue_4 (* _returnvalue_3 1000))
  ;[1 1 1] Get hit by car!
  (bind _astarget_practice_character (Utilities|Casting|CastToTargetPracticeCharacter OtherActor))
  (Character|LaunchCharacter _astarget_practice_character (Math|Vector|MakeVector (.x _returnvalue_4) (.y _returnvalue_4) (+ (.z _returnvalue_4) 5e+02)) false false)
  ;;[1 1 1] Damage Player
  (Default|ChangeHealth _astarget_practice_character (* (Variables|Default|GetCarDamage) -1)))

(event Custom|HandleCarTimer
  ;[1 1 1] BeginPlay { Create Timer & Custom Event for Handling
  (Transformation|AddActorWorldOffset (* (Variables|Default|GetDirection) (Variables|Default|GetSpeed))))

(event EventBeginPlay
  ;[1 1 1] BeginPlay { Create Timer & Custom Event for Handling
  (bind _returnvalue (Utilities|Time|SetTimerbyEvent (delegate Custom|HandleCarTimer) 0.01 true))
  (Variables|Default|SetCarTimerHandle _returnvalue)
  (Variables|Default|SetSpeed (Math|Random|RandomIntegerinRange 2 8))
  ;;[1 1 1] Damage based on Speed
  (Variables|Default|SetCarDamage (* (Variables|Default|GetSpeed) (Variables|Default|GetCarDamage))))

(fn ConstructionScript)