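; BP_CarSpawner is an actor that continuously spawns BP_Car actors within a box area.
; A looping timer started on BeginPlay spawns one car per second at a random point inside the Box component's bounds.
; Each car receives a Direction computed as the unit vector from the root to the Arrow component's location, so the Arrow's position rather than its rotation sets the heading.
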(event Custom|HandleCarSpawn
  (bind _box (Variables|Default|GetBox))
  (Game|SpawnActorfromClass "/Game/Blueprints/Car/BP_Car.BP_Car_C" (Math|Conversions|ToTransform(Vector) (Math|Random|RandomPointinBoundingBox (Transformation|GetWorldLocation _box) (Components|Box|GetScaledBoxExtent _box))) "Undefined" 0 (Math|Vector|GetUnitDirection(Vector) (Transformation|GetWorldLocation (Variables|Default|GetDefaultSceneRoot)) (Transformation|GetWorldLocation (Variables|Default|GetArrow))) 0))

(event EventBeginPlay
  (Utilities|Time|SetTimerbyEvent (delegate Custom|HandleCarSpawn) 1.0 true))

(fn ConstructionScript)