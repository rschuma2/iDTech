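; BP_Target is a shootable target that launches upward with random sideways impulse and destroys itself after two seconds.
; Construction randomizes a score Modifier and, in a separate roll, the sphere's scale; BeginPlay divides Score by that Modifier.
; A FirstPersonProjectile hit spawns an explosion with sound, adds Score to the player character and destroys the target.
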(event OnComponentHit(Sphere)
  (params (HitComponent :type Primitive%20Component%20Object%20Reference) (OtherActor :type Actor%20Object%20Reference) (OtherComp :type Primitive%20Component%20Object%20Reference) (NormalImpulse :type Vector :default "0, 0, 0") (Hit :type Hit%20Result%20Structure%20%28by%20ref%29))
  (Utilities|Casting|CastToFirstPersonProjectile OtherActor)
  (Effects|SpawnEmitteratLocation "/Game/StarterContent/Particles/P_Explosion.P_Explosion" (Transformation|GetWorldLocation (Variables|Default|GetSphere)))
  (Audio|PlaySound2D "/Game/StarterContent/Audio/Explosion01.Explosion01" 1.0 1.0 0.0 0 0)
  (bind _asfirst_person_character (Utilities|Casting|CastToFirstPersonCharacter (Game|GetPlayerCharacter 0)))
  (Default|IncreaseScore _asfirst_person_character (Variables|Default|GetScore))
  (Actor|DestroyActor))

(event Custom|DeleteTarget
  (Actor|DestroyActor))

(event EventBeginPlay
  (Physics|AddImpulse (Variables|Default|GetSphere) (Math|Vector|MakeVector (Math|Random|RandomFloatinRange -1.6e+04 1.6e+04) (Math|Random|RandomFloatinRange -1.6e+04 1.6e+04) 1e+05) "None" false)
  (Variables|Default|SetScore (Math|Float|Floor (/ (Math|Conversions|ToFloat(Integer) (Variables|Default|GetScore)) (Variables|Default|GetModifier))))
  (Utilities|Time|SetTimerbyEvent (delegate Custom|DeleteTarget) 2.0))

(fn ConstructionScript
  (bind _returnvalue (Math|Random|RandomFloatinRange 0.5 1.2))
  (bind _sphere (Variables|Default|GetSphere))
  (Variables|Default|SetModifier _returnvalue)
  (Transformation|SetWorldScale3D _sphere (* (Transformation|GetWorldScale _sphere) _returnvalue)))