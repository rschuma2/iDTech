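; BP_TargetSpawner is an actor that repeatedly spawns BP_Target actors during play.
; A looping one-second timer spawns a target slightly above the spawner, using its rotation and scale, until FirstPersonGameMode reports IsGameOver and the timer is cleared.
; A second, faster looping timer runs MoveTarget, which applies a zero world offset to the spawner itself, so it stays in place.
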(event Custom|HandleTargetSpawning
  (bind _self self)
  (bind _returnvalue (Transformation|GetActorTransform _self))
  ;[1 1 1] Handle Target Spawning
  (bind _asfirst_person_game_mode (Utilities|Casting|CastToFirstPersonGameMode (Game|GetGameMode)))
  (if (Variables|/Game/Blueprints/FirstPersonGameMode.FirstPersonGameMode_C|GetbIsGameOver _asfirst_person_game_mode)
    (Utilities|Time|ClearandInvalidateTimerbyHandle (Variables|Default|GetSpawnerHandle))
    (else
      (Game|SpawnActorfromClass "/Game/Blueprints/Targets/BP_Target.BP_Target_C" (Math|Transform|MakeTransform (Math|Vector|MakeVector (.x (.location _returnvalue)) (.y (.location _returnvalue)) (+ (.z (.location _returnvalue)) 5e+01)) (.rotation _returnvalue) (.scale _returnvalue)) "Undefined" 0 0))))

(event Custom|MoveTarget
  (Transformation|AddActorWorldOffset "0, 0, 0"))

(event EventBeginPlay
  (bind _returnvalue (Utilities|Time|SetTimerbyEvent (delegate Custom|HandleTargetSpawning) 1.0 true))
  (Variables|Default|SetSpawnerHandle _returnvalue)
  (Utilities|Time|SetTimerbyEvent (delegate Custom|MoveTarget) 0.1 true))

(fn ConstructionScript)