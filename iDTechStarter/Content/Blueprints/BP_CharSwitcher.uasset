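; BP_CharSwitcher is a trigger that switches the player to another character when a class-based character enters its box.
; On overlap, it spawns a new actor of GChar's class at the SpawnPoint actor's transform.
; It calls Possess on both player controller 0 and the spawned actor's own controller, targeting the new actor, then destroys the overlapping character.
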(event OnComponentBeginOverlap(Box)
  (params (OverlappedComponent :type Primitive%20Component%20Object%20Reference) (OtherActor :type Actor%20Object%20Reference) (OtherComp :type Primitive%20Component%20Object%20Reference) (OtherBodyIndex :type Integer) (bFromSweep :type Boolean) (SweepResult :type Hit%20Result%20Structure%20%28by%20ref%29))
  (if (Utilities|ClassIsChildOf (Utilities|GetClass OtherActor) "/Game/Blueprints/Characters/ClassBasedCharacter.ClassBasedCharacter_C")
    (bind _returnvalue (Game|SpawnActorfromClass (Utilities|GetClass (Variables|Default|GetGChar)) (Transformation|GetActorTransform (Variables|Default|GetSpawnPoint)) "Undefined" 0 0))
    (Pawn|Possess (Game|GetPlayerController 0) _returnvalue)
    (Actor|DestroyActor OtherActor)))

(fn ConstructionScript)