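; GreenCharacter is a character Blueprint whose special ability is rapid fire.
; Pressing SpecialFire passes a DoOnce gate and starts a looping timer that calls FireGun at a short fixed interval.
; Releasing the input clears the timer and resets the gate, so firing lasts only while the input is held.
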(event Custom|HandleRapidFireTimer
  ;[1 1 1] RapidFire!
  (CallFunction|FireGun))

(event EventBeginPlay
  (|CallParentFunction) ; This node is disabled and will not be called.\nDrag off pins to build functionality.
)

(event Collision|EventActorBeginOverlap
  (params (OtherActor :type Actor%20Object%20Reference)))

(event EventTick
  (params (DeltaSeconds :type Float%20%28single-precision%29)))

(event Input|ActionEvents|InputActionSpecialFire
  (params (Key :type Key%20Structure))
  ;[1 1 1] RapidFire!
  (:Pressed
    (Utilities|FlowControl|DoOnce false :!label _label
      (:Completed
        (bind _returnvalue (Utilities|Time|SetTimerbyEvent (delegate Custom|HandleRapidFireTimer) 0.1 true))
        (Variables|Default|SetRapidFireTimerHandle _returnvalue))))
  (:Released
    (Utilities|Time|ClearandInvalidateTimerbyHandle (Variables|Default|GetRapidFireTimerHandle))
    (goto _label Reset)))

(fn ConstructionScript
  (|CallParentFunction))